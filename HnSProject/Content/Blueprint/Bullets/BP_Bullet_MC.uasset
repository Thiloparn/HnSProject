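; BP_Bullet_MC is a projectile, apparently the main character's, that deals physical damage on sphere overlap and starts with its movement inactive.
; Targets implementing the damage interface need a BPC_Posture_v3: marked ones have marks consumed for summed multiplier-scaled damage, others take default damage.
; The bullet plays VFX and destroys itself on unmarked hits and non-BPI_MC obstacles, but marked hits print damage and leave it alive.
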(event OnComponentBeginOverlap(SphereCollision)
  (params (OverlappedComponent :type Primitive%20Component%20Object%20Reference) (OtherActor :type Actor%20Object%20Reference) (OtherComp :type Primitive%20Component%20Object%20Reference) (OtherBodyIndex :type Integer) (bFromSweep :type Boolean) (SweepResult :type Hit%20Result%20Structure%20%28by%20ref%29))
  (Variables|Default|SetHit%20Actor OtherActor)
  (Variables|Default|SetHitActorLocation (.Location (Collision|BreakHitResult SweepResult)))
  (if (Utilities|DoesObjectImplementInterface OtherActor (Variables|Default|GetInterfaceToDamage))
    (Utilities|IsValid (Actor|GetComponentbyClass (Variables|Default|GetHit%20Actor) "/Game/Blueprint/Components/BPC_Posture_v3.BPC_Posture_v3_C")
      (:Is%20Valid
        (if (Variables|/Game/Blueprint/Components/BPC_Posture_v3.BPC_Posture_v3_C|GetbIsMarked (Actor|GetComponentbyClass (Variables|Default|GetHit%20Actor) "/Game/Blueprint/Components/BPC_Posture_v3.BPC_Posture_v3_C"))
          (bind _consumedmarks (Default|ConsumeMark (Actor|GetComponentbyClass (Variables|Default|GetHit%20Actor) "/Game/Blueprint/Components/BPC_Posture_v3.BPC_Posture_v3_C")))
          (Variables|Default|SettotalMarkDamage 0.0)
          (for _index (range 0 (- _consumedmarks 1))
            (Variables|Default|SettotalMarkDamage (+ (Variables|Default|GettotalMarkDamage) (* (Utilities|Array|Get(acopy) (Variables|Default|GetMaksMultiplierLevels) _index) (Variables|Default|GetBulletMarkDamage)))))
          (Game|Damage|ApplyDamage (Variables|Default|GetHit%20Actor) (Variables|Default|GettotalMarkDamage) 0 self "/Game/Blueprint/BP_PhysicalDamage.BP_PhysicalDamage_C")
          (Development|PrintString (Utilities|String|ToString(Float) (Variables|Default|GettotalMarkDamage)))
          (CallFunction|PlayVFX)
          (else
            (Game|Damage|ApplyDamage (Variables|Default|GetHit%20Actor) (Variables|Default|GetBulletDefaultDamage) 0 self "/Game/Blueprint/BP_PhysicalDamage.BP_PhysicalDamage_C")
            (CallFunction|PlayVFX)
            (Actor|DestroyActor)))))
    (elif (not (Utilities|DoesObjectImplementInterface OtherActor "/Game/Blueprint/MC/BPI_MC.BPI_MC_C"))
      (CallFunction|PlayVFX)
      (Actor|DestroyActor))))

(event EventBeginPlay
  (Components|Activation|SetActive (Variables|Default|GetProjectileMovement) false false))

(fn ConstructionScript
  (|CallParentFunction))