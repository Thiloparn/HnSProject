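; BP_Bullet is a projectile actor that deals physical damage to a configurable type of pawn.
; The construction script sets the projectile movement's initial and max speed from BulletSpeed.
; A sphere overlap with a PawnToDamage actor applies damage, spawns an explosion at the sweep location and destroys the bullet, while a blocking hit only destroys it.
; A separate PlayVFX event spawns the explosion at the last stored overlap location.
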(event OnComponentHit(SphereCollision)
  (params (HitComponent :type Primitive%20Component%20Object%20Reference) (OtherActor :type Actor%20Object%20Reference) (OtherComp :type Primitive%20Component%20Object%20Reference) (NormalImpulse :type Vector :default "0, 0, 0") (Hit :type Hit%20Result%20Structure%20%28by%20ref%29))
  (Actor|DestroyActor))

(event OnComponentBeginOverlap(SphereCollision)
  (params (OverlappedComponent :type Primitive%20Component%20Object%20Reference) (OtherActor :type Actor%20Object%20Reference) (OtherComp :type Primitive%20Component%20Object%20Reference) (OtherBodyIndex :type Integer) (bFromSweep :type Boolean) (SweepResult :type Hit%20Result%20Structure%20%28by%20ref%29))
  (Variables|Default|SetHitActorLocation (.Location (Collision|BreakHitResult SweepResult)))
  (if (Class|GameplayStatics|ObjectIsA OtherActor (Variables|Default|GetPawnToDamage))
    (Game|Damage|ApplyDamage OtherActor (Variables|Default|GetBulletDefaultDamage) 0 self "/Game/Blueprint/BP_PhysicalDamage.BP_PhysicalDamage_C")
    (Effects|SpawnEmitteratLocation (Variables|Default|GetExplosionEffect) (Variables|Default|GetHitActorLocation))
    (Actor|DestroyActor)))

(event Custom|PlayVFX
  (Effects|SpawnEmitteratLocation (Variables|Default|GetExplosionEffect) (Variables|Default|GetHitActorLocation)))

(event EventBeginPlay)

(fn ConstructionScript
  (bind _projectilemovement (Variables|Default|GetProjectileMovement))
  (bind _bulletspeed (Variables|Default|GetBulletSpeed))
  (Variables|/Script/Engine.ProjectileMovementComponent|SetInitialSpeed _projectilemovement _bulletspeed)
  (Variables|/Script/Engine.ProjectileMovementComponent|SetMaxSpeed _projectilemovement _bulletspeed))