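; Camera shake Blueprint for shooting that drives location oscillation with high-frequency sine waves.
; PlayShake sets a fixed lateral oscillation on Y with zero Z amplitude.
; SetShakeDirection replaces it with a directional one, scaling the normalized 2D forward vector by AmplitudeMultiplier and mapping its X and Y to the X and Z amplitudes.
; A separate Chorra event only sets a placeholder string variable.
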(event Custom|Set%20Shake%20Direction
  (params (ForwardVector :type Vector))
  (bind _returnvalue (Class|KismetMathLibrary|VectorNormal2D ForwardVector 0.0001))
  (bind _output_get (Variables|Default|SetDesiredLocationOscillation (Math|Vector2D|MakeVector2D (* (.x _returnvalue) (Variables|Default|GetAmplitudeMultiplier)) (* (.y _returnvalue) (Variables|Default|GetAmplitudeMultiplier)))))
  (Variables|Default|SetLocOscillation (Utilities|Struct|MakeVOscillator (Utilities|Struct|MakeFOscillator (.x _output_get) 8e+01 "SineWave") "(Amplitude=0.000000,Frequency=0.000000,InitialOffset=EOO_OffsetRandom,Waveform=SineWave)" (Utilities|Struct|MakeFOscillator (.y _output_get) 8e+01 "SineWave"))))

(event Custom|Chorra
  (Variables|Default|SetNewVar "chorra"))

(event EventPlayShake
  (params (Scale :type Float%20%28single-precision%29))
  (Variables|Default|SetLocOscillation (Utilities|Struct|MakeVOscillator "(Amplitude=0.000000,Frequency=0.000000,InitialOffset=EOO_OffsetRandom,Waveform=SineWave)" (Utilities|Struct|MakeFOscillator 1e+01 8e+01 "SineWave") (Utilities|Struct|MakeFOscillator 0.0 8e+01 "SineWave"))))