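; Anim notify state that drives melee hit detection during attack animations for both enemies and, likely, the main character.
; On begin it resets the owner's hit tracking, and on each tick it asks the owner to run damage detection.
; Owners are reached through interfaces, checking BPI_Enemy_Melee first and falling back to BPI_MC_Damage, so the notify holds no detection logic itself.
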(fn ReceivedNotifyTick
  (params (MeshComp :type Skeletal%20Mesh%20Component%20Object%20Reference) (Animation :type Anim%20Sequence%20Base%20Object%20Reference) (FrameDeltaTime :type Float%20%28single-precision%29) (EventReference :type Anim%20Notify%20Event%20Reference%20Structure%20%28by%20ref%29))
  (bind _returnvalue (Components|GetOwner MeshComp))
  (if (Utilities|DoesObjectImplementInterface _returnvalue "/Game/Blueprint/Enemies/Melee/BPI_Enemy_Melee.BPI_Enemy_Melee_C")
    (Class|BPIEnemyMelee|DamageDetection(Message) _returnvalue)
    (elif (Utilities|DoesObjectImplementInterface _returnvalue "/Game/Blueprint/MC/BPI_MC_Damage.BPI_MC_Damage_C")
      (Class|BPIMCDamage|MeleeDamageDetection(Message) _returnvalue)))
  (return true))

(fn ReceivedNotifyBegin
  (params (MeshComp :type Skeletal%20Mesh%20Component%20Object%20Reference) (Animation :type Anim%20Sequence%20Base%20Object%20Reference) (TotalDuration :type Float%20%28single-precision%29) (EventReference :type Anim%20Notify%20Event%20Reference%20Structure%20%28by%20ref%29))
  (bind _returnvalue (Components|GetOwner MeshComp))
  (if (Utilities|DoesObjectImplementInterface _returnvalue "/Game/Blueprint/Enemies/Melee/BPI_Enemy_Melee.BPI_Enemy_Melee_C")
    (Class|BPIEnemyMelee|ResetHasHit(Message) _returnvalue)
    (elif (Utilities|DoesObjectImplementInterface _returnvalue "/Game/Blueprint/MC/BPI_MC_Damage.BPI_MC_Damage_C")
      (Class|BPIMCDamage|ResetHitActors(Message) _returnvalue)))
  (return true))