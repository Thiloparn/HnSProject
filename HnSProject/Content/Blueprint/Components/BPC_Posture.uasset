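; Posture component that tracks a clamped posture meter and converts a full meter into marks.
; IncreasePosture adds a set amount; reaching the maximum adds a mark and resets posture, or only prints a message once marks are capped.
; It also starts a looping timer, if none is active, intended to drain posture via DecreasePosture until zero.
; Tick prints the current posture for debugging.
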(event Custom|DecreasePosture
  (bind _output_get (Variables|Default|SetPosture (- (Variables|Default|GetPosture) 1.0)))
  (if (<= _output_get 0.0)
    (Utilities|Time|ClearandInvalidateTimerbyHandle (Variables|Default|GetDecreasePostureTimerHandle))))

(event EventTick
  (params (DeltaSeconds :type Float%20%28single-precision%29))
  (Development|PrintString (Utilities|String|ToString(Float) (Variables|Default|GetPosture)) true true "(R=0.000000,G=0.660000,B=1.000000,A=1.000000)" DeltaSeconds))

(fn DecreasePostureOvertime
  (bind _returnvalue (Utilities|Time|SetTimerbyEvent (EventDispatchers|CreateEvent :!event Custom|DecreasePosture) (Variables|Default|GetPostureDecreaseRate) true))
  (Variables|Default|SetDecreasePostureTimerHandle _returnvalue))

(fn IncreasePosture
  (bind _output_get (Variables|Default|SetPosture (Math|Float|Clamp(Float) (+ (Variables|Default|GetPostureIncrease) (Variables|Default|GetPosture)) 0.0 (Variables|Default|GetMaxPosture))))
  (if (>= _output_get (Variables|Default|GetMaxPosture))
    (CallFunction|AddMark))
  (if (not (Utilities|Time|IsTimerActivebyHandle (Variables|Default|GetDecreasePostureTimerHandle)))
    (CallFunction|DecreasePostureOvertime)))

(fn AddMark
  (if (< (Variables|Default|GetMarks) (Variables|Default|GetMaxMarks))
    (bind _result (Math|Integer|IncrementInt (Variables|Default|GetMarks))
      (:%20%20
        (Variables|Default|SetMarks _result)
        (Variables|Default|SetPosture 0.0)))
    (else
      (Development|PrintString "Maximun marks already"))))