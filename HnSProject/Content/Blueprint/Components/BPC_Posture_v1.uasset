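; Posture component that builds a capped posture meter and converts each full bar into a mark, up to a maximum, which can later be consumed.
; The per-call posture increase is read from the player character at BeginPlay.
; Increases start a looping decay timer if none is active, which is cleared once posture drains to zero.
; Mark changes update the health and posture widget and toggle the IsMarked state.
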(event Custom|DecreasePosture
  (bind _output_get (Variables|DontEdit|SetPosture (- (Variables|DontEdit|GetPosture) 1.0)))
  (if (<= _output_get 0.0)
    (Utilities|Time|ClearandInvalidateTimerbyHandle (Variables|DontEdit|GetDecreasePostureTimerHandle))))

(event EventBeginPlay
  (bind _posturedamage (Class|BPIMCDamage|GetPostureDamage(Message) (Game|GetPlayerCharacter 0)))
  (Variables|DontEdit|SetPostureIncrease _posturedamage))

(fn DecreasePostureOvertime
  (bind _returnvalue (Utilities|Time|SetTimerbyEvent (EventDispatchers|CreateEvent :!event Custom|DecreasePosture) (Variables|Edit|GetPostureDecreaseRate) true))
  (Variables|DontEdit|SetDecreasePostureTimerHandle _returnvalue))

(fn IncreasePosture
  (bind _output_get (Variables|DontEdit|SetPosture (Math|Float|Clamp(Float) (+ (Variables|DontEdit|GetPostureIncrease) (Variables|DontEdit|GetPosture)) 0.0 (Variables|Edit|GetMaxPosture))))
  (if (>= _output_get (Variables|Edit|GetMaxPosture))
    (CallFunction|AddMark))
  (if (not (Utilities|Time|IsTimerActivebyHandle (Variables|DontEdit|GetDecreasePostureTimerHandle)))
    (CallFunction|DecreasePostureOvertime)))

(fn AddMark
  (if (< (Variables|DontEdit|GetMarks) (Variables|Edit|GetMaxMarks))
    (bind _result (Math|Integer|IncrementInt (Variables|DontEdit|GetMarks))
      (:%20%20
        (Variables|DontEdit|SetMarks _result)
        (Variables|DontEdit|SetPosture 0.0)
        (Default|UpdateUIMarks (Variables|DontEdit|GetHealthNPostureWB) (Variables|DontEdit|GetMarks))
        (if (== (Variables|DontEdit|GetMarks) 1)
          (Variables|DontEdit|SetbIsMarked true))))
    (else
      (Development|PrintString "Maximun marks already"))))

(fn ConsumeMark
  (if (> (Variables|DontEdit|GetMarks) 0)
    (bind _result (Math|Integer|DecrementInt (Variables|DontEdit|GetMarks))
      (:%20%20
        (Variables|DontEdit|SetMarks _result)
        (Default|UpdateUIMarks (Variables|DontEdit|GetHealthNPostureWB) (Variables|DontEdit|GetMarks))
        (if (== (Variables|DontEdit|GetMarks) 0)
          (Variables|DontEdit|SetbIsMarked false))))))