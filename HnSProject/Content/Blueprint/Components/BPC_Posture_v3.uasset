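; Posture component that tracks stackable, expiring marks on its owner and turns them into a damage multiplier when consumed.
; AddMark adds a capped stack and restarts a retriggerable timer that expires stacks one at a time, updating the HealthNPostureWB widget's expiry animation.
; ConsumeMark sends the owner an explosion message, clears all marks and returns the summed per-stack multipliers, reusing the array's last entry for extra stacks.
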(event Custom|ResetMarks
  (Variables|DontEdit|SetMarks 0)
  (Default|ResetMarksUI (Variables|DontEdit|GetHealthNPostureWB))
  (Variables|DontEdit|SetbIsMarked false))

(event Custom|MarkTimer
  (Default|UpdateExpiredAnim (Variables|DontEdit|GetHealthNPostureWB) true)
  (Utilities|FlowControl|Sequence
    (:then_0
      (Utilities|FlowControl|RetriggerableDelay (Variables|Edit|GetMarkDuration))
      (if (> (Variables|DontEdit|GetMarks) 0)
        (Variables|DontEdit|SetMarks (Math|Integer|Max(Integer) (- (Variables|DontEdit|GetMarks) 1)))
        (Default|ExpireMarkUI (Variables|DontEdit|GetHealthNPostureWB))
        (bind _output_get (Variables|DontEdit|SetbIsMarked (> (Variables|DontEdit|GetMarks) 0)))
        (if _output_get
          (CallFunction|MarkTimer)
          (else
            (CallFunction|ResetMarks)))))
    (:then_1
      (Utilities|FlowControl|RetriggerableDelay (- (Variables|Edit|GetMarkDuration) (Variables|Edit|GetExpireAnimDuration)))
      (if (> (Variables|DontEdit|GetMarks) 0)
        (Default|UpdateExpiredAnim (Variables|DontEdit|GetHealthNPostureWB) false)))))

(event Custom|BindOnConsumeEnd
  (params (ConsumedMark :type WB%20Mark%20V%202%20Object%20Reference))
  (EventDispatchers|BindEventtoOnConsumeEnd ConsumedMark (delegate Custom|ResetMarks)))

(fn AddMark
  (CallFunction|MarkTimer)
  (if (< (Variables|DontEdit|GetMarks) (Variables|Edit|GetMaxMarks))
    (Math|Integer|IncrementInt (Variables|DontEdit|GetMarks)
      (:%20%20
        (Default|AddMarkUI (Variables|DontEdit|GetHealthNPostureWB))
        (Variables|DontEdit|SetbIsMarked true)))))

(fn ConsumeMark
  (bind _markdamagemultiplier (Variables|Edit|GetMarkDamageMultiplier))
  (if (> (Variables|DontEdit|GetMarks) 0)
    (Variables|DontEdit|SetConsumedMarks (Variables|DontEdit|GetMarks))
    (Class|BPIEnemyBase|MarkExplosion(Message) (Components|GetOwner))
    (CallFunction|ResetMarks)
    (for _index (range 0 (- (Variables|DontEdit|GetConsumedMarks) 1))
      (LocalVariables|SetTotalMultiplier (+ (LocalVariables|GetTotalMultiplier) (Utilities|Array|Get(acopy) _markdamagemultiplier (Math|Integer|Min(Integer) _index (Utilities|Array|LastIndex _markdamagemultiplier))))))
    (return (LocalVariables|GetTotalMultiplier))))