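; Posture component that manages a stack of marks on its owner and a combo multiplier level earned by consuming them.
; AddMark adds up to a cap; ConsumeMark spends one, raises the multiplier level and returns it.
; Both restart a retriggerable timer that drops marks one at a time, while a combo timer started on consume resets the level.
; HealthNPostureWB shows mark changes, a pre-expiry animation and a color update when the combo lapses.
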(event Custom|ComboTimer
  (Utilities|FlowControl|RetriggerableDelay (Variables|Edit|GetComboDuration))
  (Default|UpdateColors (Variables|DontEdit|GetHealthNPostureWB))
  (Variables|DontEdit|SetCurrentMultiplierLevel -1))

(event Custom|MarkTimer
  (Default|UpdateExpiredAnim (Variables|DontEdit|GetHealthNPostureWB) true)
  (Utilities|FlowControl|Sequence
    (:then_0
      (Utilities|FlowControl|RetriggerableDelay (Variables|Edit|GetMarkDuration))
      (bind _output_get (Variables|DontEdit|SetMarks (Math|Integer|Max(Integer) (- (Variables|DontEdit|GetMarks) 1))))
      (Default|UpdateMarksUI (Variables|DontEdit|GetHealthNPostureWB) _output_get false)
      (bind _output_get_2 (Variables|DontEdit|SetbIsMarked (> (Variables|DontEdit|GetMarks) 0)))
      (if _output_get_2
        (CallFunction|MarkTimer)))
    (:then_1
      (Utilities|FlowControl|RetriggerableDelay (- (Variables|Edit|GetMarkDuration) (Variables|Edit|GetExpireAnimDuration)))
      (Default|UpdateExpiredAnim (Variables|DontEdit|GetHealthNPostureWB) false))))

(fn AddMark
  (CallFunction|MarkTimer)
  (if (< (Variables|DontEdit|GetMarks) (Variables|Edit|GetMaxMarks))
    (bind _result (Math|Integer|IncrementInt (Variables|DontEdit|GetMarks))
      (:%20%20
        (Default|UpdateMarksUI (Variables|DontEdit|GetHealthNPostureWB) _result false)
        (Variables|DontEdit|SetbIsMarked true)))
    (else
      (Development|PrintString "Maximun marks already"))))

(fn ConsumeMark
  (if (> (Variables|DontEdit|GetMarks) 0)
    (bind _result (Math|Integer|DecrementInt (Variables|DontEdit|GetMarks))
      (:%20%20
        (Default|UpdateMarksUI (Variables|DontEdit|GetHealthNPostureWB) _result true)
        (Variables|DontEdit|SetbIsMarked (> (Variables|DontEdit|GetMarks) 0))
        (CallFunction|ComboTimer)
        (CallFunction|MarkTimer)
        (bind _result_2 (Math|Integer|IncrementInt (Variables|DontEdit|GetCurrentMultiplierLevel))
          (:%20%20
            (return _result_2)))))))