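; Level transition door that opens as an exit or swings shut on arrival when it is not an exit.
; OpenDoor waits, then a timeline rotates both leaves and fades in the floor's opacity.
; Close animates only the left leaf on a second timeline, alongside an entry transition widget at BeginPlay.
; Box overlap by a BPI_MC actor shows the game-over widget or plays an exit transition, then loads NextLevel.
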(event OnComponentBeginOverlap(Box)
  (params (OverlappedComponent :type Primitive%20Component%20Object%20Reference) (OtherActor :type Actor%20Object%20Reference) (OtherComp :type Primitive%20Component%20Object%20Reference) (OtherBodyIndex :type Integer) (bFromSweep :type Boolean) (SweepResult :type Hit%20Result%20Structure%20%28by%20ref%29))
  ;[1 1 1] Overlap
  (if (Utilities|DoesObjectImplementInterface OtherActor "/Game/Blueprint/MC/BPI_MC.BPI_MC_C")
    (if (== (Variables|Default|GetNextLevel) "GameOver")
      (bind _returnvalue (UserInterface|CreateWidget "/Game/UI/Menu/WB_GameOver.WB_GameOver_C"))
      (UserInterface|Viewport|AddtoViewport _returnvalue 0)
      (else
        (bind _returnvalue_2 (UserInterface|CreateWidget "/Game/UI/Menu/WB_MapTransition.WB_MapTransition_C" 0 true))
        (UserInterface|Viewport|AddtoViewport _returnvalue_2 0)
        (EventDispatchers|AssignOnAnimEnd _returnvalue_2 (delegate Custom|OnAnimEnd_Event))))))

(event Custom|OpenDoor
  ;[1 1 1] Open
  (Utilities|FlowControl|Delay (Variables|Default|GetOpeningDelay))
  (Components|Timeline|SetPlayRate (Variables|Default|GetTimeline) (/ 1.0 (Variables|Default|GetAnimDuration)))
  (bind _newtrack_0 (Timeline|Timeline Play)
    (:Update
      (Transformation|SetRelativeRotation (Variables|Default|GetDoorLeft) (Math|Rotator|MakeRotator 0.0 0.0 (Math|Float|Lerp 0.0 9e+01 _newtrack_0)) false false)
      (Transformation|SetRelativeRotation (Variables|Default|GetDoorRight) (Math|Rotator|MakeRotator 0.0 0.0 (* (Math|Float|Lerp 0.0 9e+01 _newtrack_0) -1.0)) false false)
      (Rendering|Material|SetScalarParameterValueonMaterials (Variables|Default|GetFloor) "Opacity" _newtrack_0))))

(event Custom|Close
  ;[1 1 1] Close
  (Components|Timeline|SetPlayRate (Variables|Default|GetTimeline) (/ 1.0 (Variables|Default|GetAnimDuration)))
  (bind _newtrack_0 (Timeline|Timeline_0 PlayFromStart)
    (:Update
      (Transformation|SetRelativeRotation (Variables|Default|GetDoorLeft) (Math|Rotator|MakeRotator 0.0 0.0 (Math|Float|Lerp -6e+01 0.0 _newtrack_0)) false false))))

(event Custom|OnAnimEnd_Event
  ;[1 1 1] Overlap
  (Game|OpenLevel(byName) (Variables|Default|GetNextLevel)))

(event EventBeginPlay
  ;[1 1 1] Begin Play
  (Rendering|Material|SetScalarParameterValueonMaterials (Variables|Default|GetFloor) "Opacity" 0.0)
  (if (not (Variables|Default|GetbIsExit))
    (CallFunction|Close)
    (bind _returnvalue (UserInterface|CreateWidget "/Game/UI/Menu/WB_MapTransition.WB_MapTransition_C"))
    (UserInterface|Viewport|AddtoViewport _returnvalue 0)))

(fn ConstructionScript)