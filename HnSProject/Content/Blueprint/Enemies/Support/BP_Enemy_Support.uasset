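; Support enemy Blueprint whose attack shields an enemy from its spawner's enemy list.
; On Attack it runs the parent attack, then rebuilds a list of enemies whose marks component reports them as marked.
; It calls SetShield on a random marked enemy, or on a random enemy from the whole list when none are marked.
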(event EventAttack
  (bind _spawner (Variables|Default|GetSpawner))
  (bind _markedenemies (Variables|Default|GetMarkedEnemies))
  (bind _enemylist (Variables|/Game/Blueprint/Enemies/BP_EnemySpawner.BP_EnemySpawner_C|GetEnemyList _spawner))
  (|CallParentFunction)
  (Utilities|Array|Clear (Variables|Default|GetMarkedEnemies))
  (for _array_element _enemylist
    (if (Variables|/Game/Blueprint/Components/BPC_Marks.BPC_Marks_C|GetbIsMarked (Variables|/Game/Blueprint/Enemies/BP_Enemy_Base.BP_Enemy_Base_C|GetBPC_Marks _array_element))
      (Utilities|Array|Add (Variables|Default|GetMarkedEnemies) _array_element)))
  (if (Utilities|Array|IsEmpty _markedenemies)
    (Default|SetShield (.OutItem (Utilities|Array|Random _enemylist)))
    (else
      (Default|SetShield (.OutItem (Utilities|Array|Random _markedenemies))))))

(fn ConstructionScript
  (|CallParentFunction))