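; BP_EnemySpawner keeps a set number of enemies alive in the level.
; On BeginPlay it fills up to SimultaneousNum, choosing melee only, ranged only or a random EnemyTypes entry, each at one of four random spawner points.
; Each enemy gets a reference to the spawner, whose OnDeath handler is bound to its health component.
; A death spawns a replacement using the last chosen type, without re-rolling it.
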(event Custom|OnDeath
  (Math|Integer|DecrementInt (Variables|Default|GetCurrentNum)
    (:%20%20
      (bind _returnvalue (Game|SpawnActorfromClass (Variables|Default|GetCurrentEnemyType) (Transformation|GetWorldTransform (Utilities|Select :Index (Math|Random|RandomIntegerinRange 0 3) :Option%200 (Variables|Default|GetSpawner1) :Option%201 (Variables|Default|GetSpawner2) :Option%202 (Variables|Default|GetSpawner3) :Option%203 (Variables|Default|GetSpawner4))) "Undefined" "MultiplyWithRoot" 0 0))
      (Variables|/Game/Blueprint/Enemies/BP_Enemy_Base.BP_Enemy_Base_C|SetSpawner _returnvalue self)
      (Math|Integer|IncrementInt (Variables|Default|GetCurrentNum)
        (:%20%20
          (EventDispatchers|BindEventtoOnDeath (Variables|/Game/Blueprint/Enemies/BP_Enemy_Base.BP_Enemy_Base_C|GetBPC_Health _returnvalue) (delegate Custom|OnDeath)))))))

(event EventBeginPlay
  (while (< (Variables|Default|GetCurrentNum) (Variables|Default|GetSimultaneousNum))
    (if (Variables|Default|GetbOnlyMelee)
      (Variables|Default|SetCurrentEnemyType "/Game/Blueprint/Enemies/Melee/BP_Enemy_Melee.BP_Enemy_Melee_C")
      (elif (Variables|Default|GetbOnlyRanged)
        (Variables|Default|SetCurrentEnemyType "/Game/Blueprint/Enemies/Ranged/BP_Enemy_Range.BP_Enemy_Range_C")
        (else
          (Variables|Default|SetCurrentEnemyType (.OutItem (Utilities|Array|Random (Variables|Default|GetEnemyTypes)))))))
    (bind _returnvalue (Game|SpawnActorfromClass (Variables|Default|GetCurrentEnemyType) (Transformation|GetWorldTransform (Utilities|Select :Index (Math|Random|RandomIntegerinRange 0 3) :Option%200 (Variables|Default|GetSpawner1) :Option%201 (Variables|Default|GetSpawner2) :Option%202 (Variables|Default|GetSpawner3) :Option%203 (Variables|Default|GetSpawner4))) "Undefined" "MultiplyWithRoot" 0 0))
    (Variables|/Game/Blueprint/Enemies/BP_Enemy_Base.BP_Enemy_Base_C|SetSpawner _returnvalue self)
    (Math|Integer|IncrementInt (Variables|Default|GetCurrentNum)
      (:%20%20
        (EventDispatchers|BindEventtoOnDeath (Variables|/Game/Blueprint/Enemies/BP_Enemy_Base.BP_Enemy_Base_C|GetBPC_Health _returnvalue) (delegate Custom|OnDeath))))))

(fn ConstructionScript)