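; BP_Enemy_Range is a ranged enemy that fires projectiles at the player.
; It extends the parent Attack event by rotating the BulletSpawn component to face the first player pawn's current location.
; It then spawns a BP_Bullet at that transform with itself as instigator and sets the bullet's TagToDamage to "MC".
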(event EventAttack
  (bind _bulletspawn (Variables|Default|GetBulletSpawn))
  (|CallParentFunction)
  (Transformation|SetWorldRotation _bulletspawn (Math|Rotator|FindLookatRotation (Transformation|GetWorldLocation _bulletspawn) (Transformation|GetActorLocation (Game|Player|GetPlayerPawn 0))) false false)
  (bind _returnvalue (Game|SpawnActorfromClass "/Game/Blueprint/Bullets/BP_Bullet.BP_Bullet_C" (Transformation|GetWorldTransform (Variables|Default|GetBulletSpawn)) "Undefined" "MultiplyWithRoot" 0 self))
  (Variables|/Game/Blueprint/Bullets/BP_Bullet.BP_Bullet_C|SetTagToDamage _returnvalue "MC"))

(fn ConstructionScript
  (|CallParentFunction))