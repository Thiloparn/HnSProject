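; Player weapon Blueprint for the main character that adds magazine ammo, fire-rate cooldown and reloading to the parent weapon's shooting.
; Shoot is gated by reload and cooldown state, calls the parent shot, restores the bullet spawn transform, spends a round and refreshes the HUD.
; An empty magazine triggers Reload, which plays the character's animation while a Timeline scaled to reload time tracks progress, then refills ammo.
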(event Custom|Reload
  ;[1 1 1] Reload
  (if (not (Variables|Default|GetisReloading))
    (bind _asbp_mccharacter (Utilities|Casting|CastToBP_MCCharacter (Actor|GetParentActor)))
    (Default|PlayReloadAnimation _asbp_mccharacter)
    (Variables|Default|SetisReloading true)
    (bind _alpha (Timeline|Timeline PlayFromStart)
      (:Update
        (Variables|Default|SetElapsedReloadTime _alpha))
      (:Finished
        (Variables|Default|SetisReloading false)
        (Variables|Default|SetCurrentNumberOfBullets (Variables|Default|GetAmmoCapacity))
        (Default|UpdateBulletDisplay (Variables|Default|GetPlayerHUD))))))

(event Custom|Cooldown
  (Utilities|FlowControl|Delay (Variables|Default|GetFireRate))
  (Variables|Default|SetbIsInFireCooldown false))

(event EventBeginPlay
  (Variables|Default|SetBulletSpawnTrasnform (Transformation|GetRelativeTransform (Variables|Default|GetSC_BulletSpawn)))
  (Variables|Default|SetCurrentNumberOfBullets (Variables|Default|GetAmmoCapacity))
  (Components|Timeline|SetPlayRate (Variables|Default|GetTimeline) (/ 1.0 (Variables|Default|GetReloadTime)))
  (bind _asbp_mccontroller (Utilities|Casting|CastToBP_MCController (Game|GetPlayerController 0)))
  (Variables|Default|SetPlayerHUD (Variables|/Game/Blueprint/MC/BP_MCController.BP_MCController_C|GetPlayerHUD _asbp_mccontroller)))

(fn ConstructionScript)

(fn SubtractBullet
  (Math|Integer|DecrementInt (Variables|Default|GetCurrentNumberOfBullets)
    (:%20%20
      (if (<= (Variables|Default|GetCurrentNumberOfBullets) 0)
        (CallFunction|Reload)))))

(fn Shoot
  (if (not (Variables|Default|GetisReloading))
    (if (not (Variables|Default|GetbIsInFireCooldown))
      (Variables|Default|SetbIsInFireCooldown true)
      (|CallParentFunction)
      (CallFunction|ResetBulletSpawn)
      (CallFunction|SubtractBullet)
      (Default|UpdateBulletDisplay (Variables|Default|GetPlayerHUD))
      (CallFunction|Cooldown)
      (return true)
      (else
        _)))
  (return false))

(fn ResetBulletSpawn
  (Transformation|SetRelativeTransform (Variables|Default|GetSC_BulletSpawn) (Variables|Default|GetBulletSpawnTrasnform) false false))

(fn GetIsReloading
  (return (Variables|Default|GetisReloading)))